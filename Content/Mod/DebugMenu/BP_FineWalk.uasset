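; BP_FineWalk is a debug menu mod component that dampens movement input on its owning CharacterZion.
; Each tick, while the DMWalk module is enabled, it reads the pending input vector from the character's movement component.
; When the Y value is near full in either direction, it adds an opposing world-Y input of 40% of that value, cutting strong input to about 60%.
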(event EventTick
  (params (DeltaSeconds :type Float%20%28single-precision%29))
  (if (Variables|/Game/Mod/DebugMenu/DebugModules/DM_Base.DM_Base_C|GetbModuleEnabled (Variables|Default|GetDM_Walk))
    (bind _ascharacter_zion (Utilities|Casting|CastToCharacterZion (Components|GetOwner)))
    (if (or (> (.y (Class|PawnMovementComponent|GetPendingInputVector (Pawn|GetMovementComponent _ascharacter_zion))) 0.9) (< (.y (Class|PawnMovementComponent|GetPendingInputVector (Pawn|GetMovementComponent _ascharacter_zion))) -0.9))
      (Class|PawnMovementComponent|AddInputVector (Pawn|GetMovementComponent _ascharacter_zion) (Math|Vector|MakeVector 0.0 (* (.y (Class|PawnMovementComponent|GetPendingInputVector (Pawn|GetMovementComponent _ascharacter_zion))) -0.4) 0.0) false))))